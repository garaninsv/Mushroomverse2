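; Tunnel spawner actor for a runner game that builds a chain of Puti tunnel segments when play begins.
; The first segment spawns at the player pawn's location, and each following one at the newest segment's SpawnPoint.
; Each spawned segment becomes the newest and receives a reference back to the spawner.
; SpawnTunnelAtSpawnPoint extends the chain by one segment per call.
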(event `self.ReceiveBeginPlay`
  (`self.SpawnInitialTunnels`))

(fn `SpawnInitialTunnels`
  (for _ (range 11)
    (`/Engine/EditorBlueprintResources/StandardMacros.IsValid` (`self.NewestTunnel`)
      (:`Is Valid`
        (`self.SpawnTunnelAtSpawnPoint`))
      (:`Is Not Valid`
        (`self.SpawnTunnel` (`self.K2_GetActorLocation` (`GameplayStatics.GetPlayerPawn` 0)))))))

(fn `SpawnTunnel`
  (params (SpawnLocation :type "Vector Structure"))
  (bind _returnvalue (`|SpawnActorFromClass` "/Game/runner/puti.puti_C" (`KismetMathLibrary.MakeTransform` SpawnLocation) "Undefined" "OverrideRootScale" null null))
  (bind _output_get (set `self.NewestTunnel` _returnvalue))
  (set `/Game/runner/puti.TunnelSpawner` self _output_get))

(fn `SpawnTunnelAtSpawnPoint`
  (`self.SpawnTunnel` (`SceneComponent.K2_GetComponentLocation` (`/Game/runner/puti.SpawnPoint` (`self.NewestTunnel`)))))

(fn `UserConstructionScript`)